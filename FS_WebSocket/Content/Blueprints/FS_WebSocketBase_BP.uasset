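; Base WebSocket Blueprint that connects the game to a local Furioos SDK socket endpoint.
; On BeginPlay it binds connect-error, connect-complete and data-received handlers, then connects to a hardcoded localhost URL.
; The handlers only print errors, connection status and incoming data to screen.
; A separate SendMessage function sends a fixed Furioos-format JSON "OK" message, but nothing in this Blueprint calls it.
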(event Custom|CE_ConnectComplete
  (Development|PrintString "Connected & Signed In" true true "(R=0.000000,G=0.660000,B=1.000000,A=1.000000)" 5.0))

(event Custom|CE_ReceiveData
  (params (data :type String))
  (Development|PrintString data true true "(R=0.000000,G=0.660000,B=1.000000,A=1.000000)" 5.0))

(event Custom|CE_ConnectError
  (params (error :type String))
  (Development|PrintString error true true "(R=0.000000,G=0.660000,B=1.000000,A=1.000000)" 5.0))

(event EventBeginPlay
  (EventDispatchers|BindEventtoFSonConnectError (delegate Custom|CE_ConnectError))
  (EventDispatchers|BindEventtoFSonConnectComplete (delegate Custom|CE_ConnectComplete))
  (EventDispatchers|BindEventtoFSonReceiveData (delegate Custom|CE_ReceiveData))
  (bind _output_get (Variables|Default|SetURL "ws://127.0.0.1:8081"))
  (Class|FSWebSocketBase|Connect _output_get))

(fn ConstructionScript)

(fn SendMessage
  (bind _output_get (Variables|Default|SetMessage "{\"type\":\"furioos\",\"task\":\"sdk\",\"data\":{\"message\":\"OK\"}}"))
  (Class|FSWebSocketBase|SendText _output_get))